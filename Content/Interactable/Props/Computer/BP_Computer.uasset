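; BP_Computer is an interactable computer prop that shows a random six-digit code and loading progress through its screen UI.
; On BeginPlay it spawns a BP_ComputerUIRenderer below itself and feeds that widget's rendered texture into a dynamic monitor material.
; Interaction events lock player move and look input and drive the loading progress.
; Completion removes the Interact tag, restores input and destroys the renderer after a short delay, while cancelling restores input and ends loading.
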(event EventBeginPlay
  ;[1 1 1] Inicjalizacja komputera
  (|CallParentFunction)
  (Variables|Default|SetCode (Math|Random|RandomIntegerinRange 100000 999999))
  (bind _returnvalue (Game|SpawnActorfromClass "/Game/Interactable/Props/Computer/Blueprints/BP_ComputerUIRenderer.BP_ComputerUIRenderer_C" (Math|Transform|MakeTransform (+ (Transformation|GetActorLocation self) "0.000000,0.000000,-1000.000000") "0, 0, 0" "1.000000,1.000000,1.000000") "AlwaysSpawn" "MultiplyWithRoot" 0 0))
  (bind _output_get (Variables|Default|SetUiRenderer _returnvalue))
  (bind _ascomputer_ui (Utilities|Casting|CastToComputerUI (UserInterface|GetWidget (Variables|/Game/Interactable/Props/Computer/Blueprints/BP_ComputerUIRenderer.BP_ComputerUIRenderer_C|GetWidget _output_get))))
  (Variables|Default|SetComputerUI _ascomputer_ui)
  (bind _texture (Default|Init (Variables|Default|GetUiRenderer)))
  (bind _returnvalue_2 (Rendering|Material|CreateDynamicMaterialInstance "/Game/Interactable/Props/Computer/Materials/Monitor.Monitor" "None" "None" :!class /Script/Engine.KismetMaterialLibrary))
  (Rendering|Material|SetTextureParameterValue _returnvalue_2 "Texture" _texture)
  (Rendering|Material|SetMaterial (Variables|Default|GetStaticMesh) 1 _returnvalue_2)
  (Default|SetCode (Variables|Default|GetComputerUI) (Variables|Default|GetCode)))

(event Collision|EventActorBeginOverlap
  (params (OtherActor :type Actor%20Object%20Reference))
  (|CallParentFunction OtherActor) ; This node is disabled and will not be called.\nDrag off pins to build functionality.
)

(event EventTick
  (params (DeltaSeconds :type Float%20%28single-precision%29))
  (|CallParentFunction DeltaSeconds) ; This node is disabled and will not be called.\nDrag off pins to build functionality.
)

(event EventInteractionStarted
  (params (Player :type BP%20Third%20Person%20Character%20Object%20Reference))
  (bind _returnvalue (Pawn|GetController Player))
  (Input|SetIgnoreMoveInput _returnvalue true)
  (Input|SetIgnoreLookInput _returnvalue true)
  (Default|StartLoading (Variables|Default|GetComputerUI)))

(event EventInteractionCanceled
  (params (Player :type BP%20Third%20Person%20Character%20Object%20Reference))
  (bind _returnvalue (Pawn|GetController Player))
  (Utilities|FlowControl|Sequence
    (:then_0
      (Input|ResetIgnoreMoveInput _returnvalue)
      (Input|ResetIgnoreLookInput _returnvalue))
    (:then_1
      (Default|EndLoading (Variables|Default|GetComputerUI)))))

(event EventInteractionTimeCompleted
  (params (Player :type BP%20Third%20Person%20Character%20Object%20Reference))
  (bind _returnvalue (Pawn|GetController Player))
  (Default|EndLoading (Variables|Default|GetComputerUI))
  (Utilities|Array|RemoveItem (Variables|Default|GetTags self) "Interact")
  (Input|ResetIgnoreMoveInput _returnvalue)
  (Input|ResetIgnoreLookInput _returnvalue)
  (Utilities|FlowControl|Delay 0.5)
  (Actor|DestroyActor (Variables|Default|GetUiRenderer)))

(event EventInteractionTimeUpdate
  (params (Time :type Float%20%28double-precision%29) (Player :type BP%20Third%20Person%20Character%20Object%20Reference))
  (Variables|/Game/Interactable/Props/Computer/UI/ComputerUI.ComputerUI_C|SetProgress (Variables|Default|GetComputerUI) (/ Time 5.0)))

(fn ConstructionScript
  (|CallParentFunction))