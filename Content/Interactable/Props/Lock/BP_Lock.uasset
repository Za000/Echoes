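; Four-dial combination lock prop that plays its opening animation when the dials match the stored combination.
; On BeginPlay it enables player input, spawns four BP_LockDial actors and attaches them to sockets on the lock mesh.
; The H, J, K and L keys each rotate one dial, then share a retriggerable half-second delay before CheckCode compares every dial's Number against LockCombination.
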(event EventBeginPlay
  (|CallParentFunction)
  (Input|EnableInput (Game|GetPlayerController 0))
  (for _index (range 0 3)
    (bind _returnvalue (Game|SpawnActorfromClass "/Game/Interactable/Props/Lock/BP_LockDial.BP_LockDial_C" (Math|Transform|MakeTransform "0, 0, 0" "0, 0, 0" "20.000000,20.000000,20.000000") "AlwaysSpawn" "MultiplyWithRoot" 0 _index 0))
    (Utilities|Array|Add (Variables|Default|GetDials) _returnvalue)
    (Transformation|AttachComponentToComponent _returnvalue (Variables|Default|GetLock) (Utilities|Select :Index _index :Option%200 "DialBone1Socket" :Option%201 "DialBone1Socket_0" :Option%202 "DialBone1Socket_1" :Option%203 "DialBone1Socket_2") "SnapToTarget" "KeepWorld" "KeepWorld" true)))

(event Collision|EventActorBeginOverlap
  (params (OtherActor :type Actor%20Object%20Reference))
  (|CallParentFunction OtherActor) ; This node is disabled and will not be called.\nDrag off pins to build functionality.
)

(event EventTick
  (params (DeltaSeconds :type Float%20%28single-precision%29))
  (|CallParentFunction DeltaSeconds) ; This node is disabled and will not be called.\nDrag off pins to build functionality.
)

(event Input|KeyboardEvents|J
  (params (Key :type Key%20Structure :default "None"))
  (:Pressed
    (Default|RotateDial (Utilities|Array|Get(acopy) (Variables|Default|GetDials) 1))
    (Utilities|FlowControl|RetriggerableDelay 0.5)
    (bind _success (CallFunction|CheckCode))
    (if _success
      (Components|Animation|PlayAnimation (Variables|Default|GetLock) "/Game/Interactable/Props/Lock/LockOpen.LockOpen" false))))

(event Input|KeyboardEvents|H
  (params (Key :type Key%20Structure :default "None"))
  (:Pressed
    (Default|RotateDial (Utilities|Array|Get(acopy) (Variables|Default|GetDials)))
    (Utilities|FlowControl|RetriggerableDelay 0.5)
    (bind _success (CallFunction|CheckCode))
    (if _success
      (Components|Animation|PlayAnimation (Variables|Default|GetLock) "/Game/Interactable/Props/Lock/LockOpen.LockOpen" false))))

(event Input|KeyboardEvents|K
  (params (Key :type Key%20Structure :default "None"))
  (:Pressed
    (Default|RotateDial (Utilities|Array|Get(acopy) (Variables|Default|GetDials) 2))
    (Utilities|FlowControl|RetriggerableDelay 0.5)
    (bind _success (CallFunction|CheckCode))
    (if _success
      (Components|Animation|PlayAnimation (Variables|Default|GetLock) "/Game/Interactable/Props/Lock/LockOpen.LockOpen" false))))

(event Input|KeyboardEvents|L
  (params (Key :type Key%20Structure :default "None"))
  (:Pressed
    (Default|RotateDial (Utilities|Array|Get(acopy) (Variables|Default|GetDials) 3))
    (Utilities|FlowControl|RetriggerableDelay 0.5)
    (bind _success (CallFunction|CheckCode))
    (if _success
      (Components|Animation|PlayAnimation (Variables|Default|GetLock) "/Game/Interactable/Props/Lock/LockOpen.LockOpen" false))))

(fn ConstructionScript
  (|CallParentFunction))

(fn CheckCode
  (bind (_array_element _array_index) (Utilities|Array|ForEachLoopwithBreak (Variables|Default|GetDials) :!label _label)
    (:LoopBody
      (if (== (Utilities|Array|Get(acopy) (Variables|Default|GetLockCombination) _array_index) (Variables|/Game/Interactable/Props/Lock/BP_LockDial.BP_LockDial_C|GetNumber _array_element))
        (LocalVariables|SetLocalSuccess true)
        (else
          (LocalVariables|SetLocalSuccess false)
          (goto _label Break))))
    (:Completed
      (return (LocalVariables|GetLocalSuccess)))))