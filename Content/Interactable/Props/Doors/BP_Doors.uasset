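; BP_Doors is an interactable door that a player swings open or closed with horizontal mouse movement.
; Each interaction update multicasts the instigator and sends the player's mouse X to a server event.
; That event adds the sensitivity-scaled input to the door's relative yaw, floors it at zero and applies it through MoveDoor.
; Helper events toggle player move and look input, and cancelling calls the reset and clears the interacting player.
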(event Custom|MoveDoor
  (params (Ammount :type Float%20%28double-precision%29))
  (Transformation|SetRelativeRotation (Variables|Default|GetDoor) (Math|Rotator|MakeRotator 0.0 0.0 Ammount) false false))

(event Custom|IgnorePlayerInputs
  (params (Player :type BP%20Third%20Person%20Character%20Object%20Reference))
  (bind _returnvalue (Pawn|GetController Player))
  (Input|SetIgnoreMoveInput _returnvalue true)
  (Input|SetIgnoreLookInput _returnvalue true))

(event Custom|ResetPlayerInputs
  (params (Player :type BP%20Third%20Person%20Character%20Object%20Reference))
  (bind _returnvalue (Pawn|GetController Player))
  (Utilities|IsValid Player
    (:Is%20Valid
      (Input|ResetIgnoreMoveInput _returnvalue)
      (Input|ResetIgnoreLookInput _returnvalue))))

(event Custom|Door%20Action_RunOnServer
  (params (Ammount :type Float%20%28double-precision%29))
  (CallFunction|MoveDoor (Math|Float|Max(Float) (.Yaw (Math|Rotator|BreakRotator (Math|Rotator|CombineRotators (Variables|/Script/Engine.SceneComponent|GetRelativeRotation (Variables|Default|GetDoor)) (Math|Rotator|MakeRotator 0.0 0.0 (* Ammount (Variables|Default|GetSens)))))) 0.0)))

(event Custom|SetInstigator_multicast
  (params (Instigator :type Pawn%20Object%20Reference))
  (Variables|Default|SetInstigator Instigator))

(event EventBeginPlay
  (|CallParentFunction) ; This node is disabled and will not be called.\nDrag off pins to build functionality.
)

(event Collision|EventActorBeginOverlap
  (params (OtherActor :type Actor%20Object%20Reference))
  (|CallParentFunction OtherActor) ; This node is disabled and will not be called.\nDrag off pins to build functionality.
)

(event EventTick
  (params (DeltaSeconds :type Float%20%28single-precision%29))
  (|CallParentFunction DeltaSeconds) ; This node is disabled and will not be called.\nDrag off pins to build functionality.
)

(event EventInteractionCanceled
  (params (Player :type BP%20Third%20Person%20Character%20Object%20Reference))
  (CallFunction|ResetPlayerInputs)
  (Variables|Default|SetInteractedPlayer 0))

(event EventInteractionUpdate
  (params (Player :type BP%20Third%20Person%20Character%20Object%20Reference))
  (CallFunction|SetInstigatorMulticast Player)
  (CallFunction|DoorActionRunonServer (Variables|/Game/ThirdPerson/Blueprints/BP_ThirdPersonCharacter.BP_ThirdPersonCharacter_C|GetPlayerMouseX Player)))

(fn ConstructionScript
  (|CallParentFunction))

(fn OnRepPlayerMousePosition)